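; BP_Bones is a collectible bone pickup that adds its BonesAmount to the game mode's bone count.
; Touching the OverlapBone component plays a pickup sound, credits the bones and destroys the actor, unless it is already moving.
; If the player has the first power-up, entering OverlapMagnet starts a timeline that lerps the bone to the player while shrinking it, then collects it without the sound.
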(event OnComponentBeginOverlap(OverlapBone)
  (params (OverlappedComponent :type Primitive%20Component%20Object%20Reference) (OtherActor :type Actor%20Object%20Reference) (OtherComp :type Primitive%20Component%20Object%20Reference) (OtherBodyIndex :type Integer) (bFromSweep :type Boolean) (SweepResult :type Hit%20Result%20Structure%20%28by%20ref%29))
  (bind _asbp_third_person_character (Utilities|Casting|CastToBP_ThirdPersonCharacter OtherActor))
  (if (not (Variables|Default|GetMoving))
    (Variables|Default|SetAs%20BP%20Third%20Person%20Character _asbp_third_person_character)
    (Audio|PlaySound2D "/Game/Audio/BonePickUp.BonePickUp" 0.5 1.0 0.0 0 0)
    (CallFunction|IncreaseandDestroy)))

(event OnComponentBeginOverlap(OverlapMagnet)
  (params (OverlappedComponent :type Primitive%20Component%20Object%20Reference) (OtherActor :type Actor%20Object%20Reference) (OtherComp :type Primitive%20Component%20Object%20Reference) (OtherBodyIndex :type Integer) (bFromSweep :type Boolean) (SweepResult :type Hit%20Result%20Structure%20%28by%20ref%29))
  (bind _asbp_third_person_character (Utilities|Casting|CastToBP_ThirdPersonCharacter OtherActor))
  (if (Utilities|Array|Get(acopy) (Variables|/Game/ThirdPerson/Blueprints/BP_ThirdPersonCharacter.BP_ThirdPersonCharacter_C|GetPower_Ups _asbp_third_person_character))
    (Variables|Default|SetAs%20BP%20Third%20Person%20Character _asbp_third_person_character)
    (Variables|Default|SetMoving true)
    (CallFunction|MoveCointoPlayer)))

(event Custom|Increase%20And%20Destroy
  (Default|IncreaseBones (Variables|/Game/ThirdPerson/Blueprints/BP_ThirdPersonCharacter.BP_ThirdPersonCharacter_C|GetGameModeRef (Variables|Default|GetAs%20BP%20Third%20Person%20Character)) (Variables|Default|GetBones%20Amount))
  (Actor|DestroyActor))

(event Custom|MoveCoinToPlayer
  (Variables|Default|SetStartLocation (Transformation|GetActorLocation))
  (bind _coin (Timeline|TL_MoveC PlayFromStart)
    (:Update
      (Transformation|SetWorldLocation (Variables|Default|GetDefaultSceneRoot) (Math|Vector|Lerp(Vector) (Variables|Default|GetStartLocation) (Transformation|GetWorldLocation (Variables|/Script/Engine.Character|GetCapsuleComponent (Variables|Default|GetAs%20BP%20Third%20Person%20Character))) _coin) false false)
      (Transformation|SetRelativeScale3D (Variables|Default|GetBone) (Math|Vector|Lerp(Vector) "0.200000,0.200000,0.200000" "0, 0, 0" _coin)))
    (:Finished
      (CallFunction|IncreaseandDestroy))))

(event EventBeginPlay)

(event Collision|EventActorBeginOverlap
  (params (OtherActor :type Actor%20Object%20Reference)))

(event EventTick
  (params (DeltaSeconds :type Float%20%28single-precision%29)))

(fn ConstructionScript)