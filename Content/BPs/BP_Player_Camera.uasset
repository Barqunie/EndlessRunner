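; Player camera for a three-lane game that follows the player along X and shifts sideways between lanes.
; Each Tick it moves its camera component to the player capsule's X plus the FollowLocation X offset, with height taken from FollowLocation.
; CalculateLaneLocation maps LaneIndex to left, centre or right by MoveAmount and eases the camera's Y toward it with FInterpTo.
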(event EventBeginPlay)

(event Collision|EventActorBeginOverlap
  (params (OtherActor :type Actor%20Object%20Reference)))

(event EventTick
  (params (DeltaSeconds :type Float%20%28single-precision%29))
  (bind _followlocation (Variables|Default|GetFollowLocation))
  (Transformation|SetWorldLocation (Variables|CameraActor|GetCameraComponent) (Math|Vector|MakeVector (+ (.x (Transformation|GetWorldLocation (Variables|/Script/Engine.Character|GetCapsuleComponent (Variables|Default|GetPlayerRef)))) (.x (.location _followlocation))) (CallFunction|CalculateLaneLocation) (.z (.location _followlocation))) false false))

(fn ConstructionScript)

(fn CalculateLaneLocation
  (bind _moveamount (Variables|Default|GetMoveAmount))
  (return (Math|Interpolation|FInterpTo (.y (Transformation|GetWorldLocation (Variables|CameraActor|GetCameraComponent))) (Utilities|Select :Index (Variables|Default|GetLaneIndex) :Option%200 (* _moveamount -1.0) :Option%201 0.0 :Option%202 _moveamount) (Utilities|Time|GetWorldDeltaSeconds) 8.0)))