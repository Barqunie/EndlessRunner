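; BP_Cage is an endless runner obstacle that the player opens with a key or dies on touching.
; On BeginPlay it caches the game mode and randomizes the skeletal mesh's looping animation and material.
; On DeathCollision overlap, a player with keys spends one, destroying the cage mesh with a sound, updating the game mode's key count and awarding bones before the actor is destroyed.
; Without keys, the overlap calls the character's Death.
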(event OnComponentBeginOverlap(DeathCollision)
  (params (OverlappedComponent :type Primitive%20Component%20Object%20Reference) (OtherActor :type Actor%20Object%20Reference) (OtherComp :type Primitive%20Component%20Object%20Reference) (OtherBodyIndex :type Integer) (bFromSweep :type Boolean) (SweepResult :type Hit%20Result%20Structure%20%28by%20ref%29))
  (bind _as_gm_endless_runner (Variables|Default|GetAs%20GM%20Endless%20Runner))
  (bind _asbp_third_person_character (Utilities|Casting|CastToBP_ThirdPersonCharacter OtherActor))
  (if (>= (Variables|/Game/ThirdPerson/Blueprints/BP_ThirdPersonCharacter.BP_ThirdPersonCharacter_C|GetKeys _asbp_third_person_character) 1)
    (Components|DestroyComponent (Variables|Default|GetCage))
    (Audio|PlaySoundatLocation "/Game/Audio/CageOpenSound.CageOpenSound" (Transformation|GetActorLocation) "0, 0, 0" 1.0 1.0 0.0 0 0 0 0)
    (bind _result (Math|Integer|DecrementInt (Variables|/Game/ThirdPerson/Blueprints/BP_ThirdPersonCharacter.BP_ThirdPersonCharacter_C|GetKeys _asbp_third_person_character))
      (:%20%20
        (Default|IncreaseKeys _as_gm_endless_runner _result)
        (Default|IncreaseBones _as_gm_endless_runner 5)
        (Utilities|FlowControl|Delay 1.0)
        (Actor|DestroyActor)))
    (else
      (Default|Death _asbp_third_person_character))))

(event EventBeginPlay
  (bind _skeletalmesh (Variables|Default|GetSkeletalMesh))
  (bind _skeletalmesh_2 (Variables|Default|GetSkeletalMesh))
  (bind _asgm_endless_runner (Utilities|Casting|CastToGM_Endless_Runner (Game|GetGameMode)))
  (Variables|Default|SetAs%20GM%20Endless%20Runner _asgm_endless_runner)
  (switch int (Math|Random|RandomIntegerinRange 0 2)
    (:0
      (Components|Animation|PlayAnimation _skeletalmesh 0 true))
    (:1
      (Components|Animation|PlayAnimation _skeletalmesh 0 true))
    (:2
      (Components|Animation|PlayAnimation _skeletalmesh 0 true)))
  (switch int (Math|Random|RandomIntegerinRange 0 2)
    (:0
      (Rendering|Material|SetMaterial _skeletalmesh_2 0 0))
    (:1
      (Rendering|Material|SetMaterial _skeletalmesh_2 0 0))
    (:2
      (Rendering|Material|SetMaterial _skeletalmesh_2 0 0))))

(event Collision|EventActorBeginOverlap
  (params (OtherActor :type Actor%20Object%20Reference)))

(event EventTick
  (params (DeltaSeconds :type Float%20%28single-precision%29)))

(fn ConstructionScript)