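; Drone enemy that faces the player, fires projectiles with a laser sound, and destroys itself after a few shots.
; Looping timers started on BeginPlay drive the firing and switch its point light between blue and red.
; Tick smoothly rotates it toward the cached player character and pushes it along world X by a fixed per-frame step, regardless of facing or frame rate.
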(event Custom|Fire
  (Game|SpawnActorfromClass "/Game/BPs/BP_Projectile.BP_Projectile_C" (Transformation|GetActorTransform) "Undefined" "MultiplyWithRoot" 0 0)
  (Audio|PlaySound2D "/Engine/VREditor/Sounds/UI/Laser_Push.Laser_Push" 3.0 1.0 0.0 0 0)
  (if (>= (Variables|Default|GetShootcount) 3)
    (Actor|DestroyActor)
    (else
      (Math|Integer|IncrementInt (Variables|Default|GetShootcount)))))

(event Custom|LightChange
  (Rendering|Components|Light|SetLightColor (Variables|Default|GetPointLight) "(R=0.000000,G=0.095112,B=1.000000,A=1.000000)" true)
  (Utilities|FlowControl|Delay 0.5)
  (Rendering|Components|Light|SetLightColor (Variables|Default|GetPointLight) "(R=0.744792,G=0.006905,B=0.000000,A=1.000000)" true))

(event EventBeginPlay
  (Utilities|Time|SetTimerbyEvent (delegate Custom|Fire) 1.0 true)
  (bind _asbp_third_person_character (Utilities|Casting|CastToBP_ThirdPersonCharacter (Game|GetPlayerCharacter 0)))
  (Variables|Default|SetAs%20BP%20Third%20Person%20Character _asbp_third_person_character)
  (Utilities|Time|SetTimerbyEvent (delegate Custom|LightChange) 0.5 true))

(event Collision|EventActorBeginOverlap
  (params (OtherActor :type Actor%20Object%20Reference)))

(event EventTick
  (params (DeltaSeconds :type Float%20%28single-precision%29))
  (Transformation|SetActorRotation (Math|Interpolation|RInterpTo (Transformation|GetActorRotation) (Math|Rotator|FindLookatRotation (Transformation|GetActorLocation) (Transformation|GetActorLocation (Variables|Default|GetAs%20BP%20Third%20Person%20Character))) (Utilities|Time|GetWorldDeltaSeconds) 5.0))
  (Transformation|AddActorWorldOffset "5.000000,0.000000,0.000000"))

(fn ConstructionScript)