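; Base track tile that dresses itself with random scenery and drives continuous tile spawning as the player moves.
; On BeginPlay, it fills left and right rows of spawn points with randomly picked child actor components at each point's relative transform.
; When the third-person character overlaps SpawnBox, it asks the game mode to spawn tiles.
; When the character overlaps DestroyBox, the tile destroys itself.
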(event OnComponentBeginOverlap(SpawnBox)
  (params (OverlappedComponent :type Primitive%20Component%20Object%20Reference) (OtherActor :type Actor%20Object%20Reference) (OtherComp :type Primitive%20Component%20Object%20Reference) (OtherBodyIndex :type Integer) (bFromSweep :type Boolean) (SweepResult :type Hit%20Result%20Structure%20%28by%20ref%29))
  (Utilities|Casting|CastToBP_ThirdPersonCharacter OtherActor)
  (Default|SpawnTile (Variables|Default|GetGameModeRef) 2))

(event OnComponentBeginOverlap(DestroyBox)
  (params (OverlappedComponent :type Primitive%20Component%20Object%20Reference) (OtherActor :type Actor%20Object%20Reference) (OtherComp :type Primitive%20Component%20Object%20Reference) (OtherBodyIndex :type Integer) (bFromSweep :type Boolean) (SweepResult :type Hit%20Result%20Structure%20%28by%20ref%29))
  (Utilities|Casting|CastToBP_ThirdPersonCharacter OtherActor)
  (Actor|DestroyActor))

(event EventBeginPlay
  (CallFunction|SpawnEnviroment))

(event Collision|EventActorBeginOverlap
  (params (OtherActor :type Actor%20Object%20Reference)))

(event EventTick
  (params (DeltaSeconds :type Float%20%28single-precision%29)))

(fn ConstructionScript)

(fn SpawnEnviroment
  (Utilities|FlowControl|Sequence
    (:then_0
      (Utilities|FlowControl|Sequence
        (:then_0
          (Variables|Default|SetEnvSpawnTranfsorm (Transformation|GetRelativeTransform (Variables|Default|GetEnvSpawnPointL1)))
          (CallFunction|RandomEnvSpawner))
        (:then_1
          (Variables|Default|SetEnvSpawnTranfsorm (Transformation|GetRelativeTransform (Variables|Default|GetEnvSpawnPointL2)))
          (CallFunction|RandomEnvSpawner))
        (:then_2
          (Variables|Default|SetEnvSpawnTranfsorm (Transformation|GetRelativeTransform (Variables|Default|GetEnvSpawnPointL3)))
          (CallFunction|RandomEnvSpawner))
        (:then_3
          (Variables|Default|SetEnvSpawnTranfsorm (Transformation|GetRelativeTransform (Variables|Default|GetEnvSpawnPointL4)))
          (CallFunction|RandomEnvSpawner))
        (:then_4
          (Variables|Default|SetEnvSpawnTranfsorm (Transformation|GetRelativeTransform (Variables|Default|GetEnvSpawnPointL5)))
          (CallFunction|RandomEnvSpawner))))
    (:then_1
      (Utilities|FlowControl|Sequence
        (:then_0
          (Variables|Default|SetEnvSpawnTranfsorm (Transformation|GetRelativeTransform (Variables|Default|GetEnvSpawnPointR1)))
          (CallFunction|RandomEnvSpawner))
        (:then_1
          (Variables|Default|SetEnvSpawnTranfsorm (Transformation|GetRelativeTransform (Variables|Default|GetEnvSpawnPointR2)))
          (CallFunction|RandomEnvSpawner))
        (:then_2
          (Variables|Default|SetEnvSpawnTranfsorm (Transformation|GetRelativeTransform (Variables|Default|GetEnvSpawnPointR3)))
          (CallFunction|RandomEnvSpawner))
        (:then_3
          (Variables|Default|SetEnvSpawnTranfsorm (Transformation|GetRelativeTransform (Variables|Default|GetEnvSpawnPointR4)))
          (CallFunction|RandomEnvSpawner))
        (:then_4
          (Variables|Default|SetEnvSpawnTranfsorm (Transformation|GetRelativeTransform (Variables|Default|GetEnvSpawnPointR5)))
          (CallFunction|RandomEnvSpawner))))))

(fn RandomEnvSpawner
  (switch int (Math|Random|RandomIntegerinRange 0 5)
    (:0
      (AddComponent|AddChildActorComponent false (Variables|Default|GetEnvSpawnTranfsorm)))
    (:1
      (AddComponent|AddChildActorComponent false (Variables|Default|GetEnvSpawnTranfsorm)))
    (:2
      (AddComponent|AddChildActorComponent false (Variables|Default|GetEnvSpawnTranfsorm)))
    (:3
      (AddComponent|AddChildActorComponent false (Variables|Default|GetEnvSpawnTranfsorm)))
    (:4
      (AddComponent|AddChildActorComponent false (Variables|Default|GetEnvSpawnTranfsorm)))
    (:5
      (AddComponent|AddChildActorComponent false (Variables|Default|GetEnvSpawnTranfsorm)))))