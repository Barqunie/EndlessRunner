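; Intersection road tile that requests a tile spawn from the game mode and destroys itself as the player crosses its trigger boxes.
; BeginPlay attaches random child-actor scenery at six side points and randomly sets the traffic light, favoring red.
; A player trigger starts cross traffic: red loops randomly timed moving cars via delayed recursion, green places optional cars at the light.
; Side collision volumes destroy horizontal cars that reach them.
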(event OnComponentBeginOverlap(SpawnBox)
  (params (OverlappedComponent :type Primitive%20Component%20Object%20Reference) (OtherActor :type Actor%20Object%20Reference) (OtherComp :type Primitive%20Component%20Object%20Reference) (OtherBodyIndex :type Integer) (bFromSweep :type Boolean) (SweepResult :type Hit%20Result%20Structure%20%28by%20ref%29))
  (Utilities|Casting|CastToBP_ThirdPersonCharacter OtherActor)
  (Default|SpawnTile (Variables|Default|GetGameModeRef) 2))

(event OnComponentBeginOverlap(DestroyBox)
  (params (OverlappedComponent :type Primitive%20Component%20Object%20Reference) (OtherActor :type Actor%20Object%20Reference) (OtherComp :type Primitive%20Component%20Object%20Reference) (OtherBodyIndex :type Integer) (bFromSweep :type Boolean) (SweepResult :type Hit%20Result%20Structure%20%28by%20ref%29))
  (Utilities|Casting|CastToBP_ThirdPersonCharacter OtherActor)
  (Actor|DestroyActor))

(event OnComponentBeginOverlap(CarSpawnCollision)
  (params (OverlappedComponent :type Primitive%20Component%20Object%20Reference) (OtherActor :type Actor%20Object%20Reference) (OtherComp :type Primitive%20Component%20Object%20Reference) (OtherBodyIndex :type Integer) (bFromSweep :type Boolean) (SweepResult :type Hit%20Result%20Structure%20%28by%20ref%29))
  (Utilities|Casting|CastToBP_ThirdPersonCharacter OtherActor)
  (CallFunction|SpawnCar))

(event OnComponentBeginOverlap(CarDestroyCollisionL)
  (params (OverlappedComponent :type Primitive%20Component%20Object%20Reference) (OtherActor :type Actor%20Object%20Reference) (OtherComp :type Primitive%20Component%20Object%20Reference) (OtherBodyIndex :type Integer) (bFromSweep :type Boolean) (SweepResult :type Hit%20Result%20Structure%20%28by%20ref%29))
  (bind _asmoving_car_horizontal (Utilities|Casting|CastToMoving_Car_Horizontal OtherActor))
  (Actor|DestroyActor _asmoving_car_horizontal))

(event OnComponentBeginOverlap(CarDestroyCollisionR)
  (params (OverlappedComponent :type Primitive%20Component%20Object%20Reference) (OtherActor :type Actor%20Object%20Reference) (OtherComp :type Primitive%20Component%20Object%20Reference) (OtherBodyIndex :type Integer) (bFromSweep :type Boolean) (SweepResult :type Hit%20Result%20Structure%20%28by%20ref%29))
  (bind _asmoving_car_horizontal (Utilities|Casting|CastToMoving_Car_Horizontal OtherActor))
  (Actor|DestroyActor _asmoving_car_horizontal))

(event Custom|SpawnCar
  (if (not (Variables|Default|GetLightGreen))
    (CallFunction|SpawnRandomTrafficHorizontal)
    (Utilities|FlowControl|Delay (Math|Random|RandomFloatinRange 2.0 4.0))
    (CallFunction|SpawnCar)
    (else
      (CallFunction|SpawnRandomTrafficatLight))))

(event EventBeginPlay
  (CallFunction|SpawnEnviroment)
  (CallFunction|SetTrafficLight))

(event Collision|EventActorBeginOverlap
  (params (OtherActor :type Actor%20Object%20Reference)))

(event EventTick
  (params (DeltaSeconds :type Float%20%28single-precision%29)))

(fn ConstructionScript)

(fn SpawnEnviroment
  (Utilities|FlowControl|Sequence
    (:then_0
      (Utilities|FlowControl|Sequence
        (:then_0
          (Variables|Default|SetEnvSpawnTranfsorm (Transformation|GetRelativeTransform (Variables|Default|GetEnvSpawnPointL1)))
          (CallFunction|RandomEnvSpawner))
        (:then_1
          (Variables|Default|SetEnvSpawnTranfsorm (Transformation|GetRelativeTransform (Variables|Default|GetEnvSpawnPointL2)))
          (CallFunction|RandomEnvSpawner))
        (:then_2
          (Variables|Default|SetEnvSpawnTranfsorm (Transformation|GetRelativeTransform (Variables|Default|GetEnvSpawnPointL3)))
          (CallFunction|RandomEnvSpawner))))
    (:then_1
      (Utilities|FlowControl|Sequence
        (:then_0
          (Variables|Default|SetEnvSpawnTranfsorm (Transformation|GetRelativeTransform (Variables|Default|GetEnvSpawnPointR1)))
          (CallFunction|RandomEnvSpawner))
        (:then_1
          (Variables|Default|SetEnvSpawnTranfsorm (Transformation|GetRelativeTransform (Variables|Default|GetEnvSpawnPointR2)))
          (CallFunction|RandomEnvSpawner))
        (:then_2
          (Variables|Default|SetEnvSpawnTranfsorm (Transformation|GetRelativeTransform (Variables|Default|GetEnvSpawnPointR3)))
          (CallFunction|RandomEnvSpawner))))))

(fn RandomEnvSpawner
  (switch int (Math|Random|RandomIntegerinRange 0 5)
    (:0
      (AddComponent|AddChildActorComponent false (Variables|Default|GetEnvSpawnTranfsorm)))
    (:1
      (AddComponent|AddChildActorComponent false (Variables|Default|GetEnvSpawnTranfsorm)))
    (:2
      (AddComponent|AddChildActorComponent false (Variables|Default|GetEnvSpawnTranfsorm)))
    (:3
      (AddComponent|AddChildActorComponent false (Variables|Default|GetEnvSpawnTranfsorm)))
    (:4
      (AddComponent|AddChildActorComponent false (Variables|Default|GetEnvSpawnTranfsorm)))
    (:5
      (AddComponent|AddChildActorComponent false (Variables|Default|GetEnvSpawnTranfsorm)))))

(fn SpawnRandomTrafficHorizontal
  (Variables|Default|SetCarSpeed (Math|Random|RandomFloatinRange 1e+01 15.0))
  (switch int (Math|Random|RandomIntegerinRange 0 2)
    (:0
      (Game|SpawnActorfromClass "/Game/BPs/Obstacles/Moving_Car_Horizontal.Moving_Car_Horizontal_C" (Transformation|GetWorldTransform (Variables|Default|GetCarSpawnL1)) "Undefined" "MultiplyWithRoot" 0 true (Variables|Default|GetCarSpeed) 0))
    (:1
      (Game|SpawnActorfromClass "/Game/BPs/Obstacles/Moving_Car_Horizontal.Moving_Car_Horizontal_C" (Transformation|GetWorldTransform (Variables|Default|GetCarSpawnR1)) "Undefined" "MultiplyWithRoot" 0 true (* (Variables|Default|GetCarSpeed) -1.0) 0))
    (:2
      (Game|SpawnActorfromClass "/Game/BPs/Obstacles/Moving_Car_Horizontal.Moving_Car_Horizontal_C" (Transformation|GetWorldTransform (Variables|Default|GetCarSpawnR2)) "Undefined" "MultiplyWithRoot" 0 true (* (Variables|Default|GetCarSpeed) -1.0) 0))))

(fn SetTrafficLight
  (if (< (Math|Random|RandomFloatinRange 0.0 1.0) 0.4)
    (Variables|Default|SetLightGreen true)
    (Rendering|SetVisibility (Variables|Default|GetRedLightL) false false)
    (Rendering|SetVisibility (Variables|Default|GetGreenLightL) true false)
    (else
      (Variables|Default|SetLightGreen false))))

(fn SpawnRandomTrafficatLight
  (Utilities|FlowControl|Sequence
    (:then_0
      (if (Math|Random|RandomBool)
        (Game|SpawnActorfromClass "/Game/BPs/Obstacles/Moving_Car_Horizontal.Moving_Car_Horizontal_C" (Transformation|GetWorldTransform (Variables|Default|GetCarSpawnAtLight_R)) "Undefined" "MultiplyWithRoot" 0 false 0.0 0)))
    (:then_1
      (if (Math|Random|RandomBool)
        (Game|SpawnActorfromClass "/Game/BPs/Obstacles/Moving_Car_Horizontal.Moving_Car_Horizontal_C" (Transformation|GetWorldTransform (Variables|Default|GetCarSpawnAtLight_R1)) "Undefined" "MultiplyWithRoot" 0 false 0.0 0)))
    (:then_2
      (if (Math|Random|RandomBool)
        (Game|SpawnActorfromClass "/Game/BPs/Obstacles/Moving_Car_Horizontal.Moving_Car_Horizontal_C" (Transformation|GetWorldTransform (Variables|Default|GetCarSpawnAtLight_L)) "Undefined" "MultiplyWithRoot" 0 false 0.0 0)))))